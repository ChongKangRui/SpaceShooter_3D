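; BP_AIShip_Simulation is an AI ship that simulates movement by pathfinding to a random location.
; One second after BeginPlay, if ShouldSimulate is set, MoveNewRandomLocation picks a point on the AgentComponent's grid within a distance band around the ship and calls MoveTo.
; The pathfinding state-change switch leads nowhere and a further move call is unwired, so the ship does not chain moves.
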(event `self.ReceiveBeginPlay`
  (`KismetSystemLibrary.Delay` 1.0)
  (if (`self.ShouldSimulate`)
    (`self.MoveNewRandomLocation`)))

(event `MoveNewRandomLocation`
  (bind _agentcomponent (`self.AgentComponent`))
  (`AStarAgentComponent.MoveTo` _agentcomponent (`AStarPathGrid.GetRandomLocationWithinRange` (`AStarAgentComponent.GetGridReference` _agentcomponent) (`self.K2_GetActorLocation`) 2000.0 7000.0)))

(event `self.ReceiveTick`
  (params (DeltaSeconds :type "Float (single-precision)")))

(event `self.AgentComponent.OnPathfindingStateChanged`
  (params (AgentStatus :type "EPathfindingStatus Enum" :default "None"))
  (switch `EPathfindingStatus` AgentStatus))

(fn `UserConstructionScript`)