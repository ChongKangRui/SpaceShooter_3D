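; Base Blueprint for a ship mesh actor that runs as a child of an owning actor.
; Damage it receives is re-applied to the parent actor with the same instigator, causer and damage type.
; Each Tick, it maps the speed of the parent's CharacterMovementComponent to a clamped BurstAlpha value, which nothing in this Blueprint consumes.
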(event `self.ReceiveBeginPlay`
  (add `self.OnTakeAnyDamage` (delegate `OnTakeAnyDamage_Event`))
  (set `self.OwnerCharMovementComp` (`self.GetComponentByClass` (`self.GetParentActor`) "/Script/Engine.CharacterMovementComponent")))

(event `OnTakeAnyDamage_Event` :!signature `self.OnTakeAnyDamage`
  (params (DamagedActor :type "Actor Object Reference") (Damage :type "Float (single-precision)") (DamageType :type "DamageType Object Reference") (InstigatedBy :type "Controller Object Reference") (DamageCauser :type "Actor Object Reference"))
  (`GameplayStatics.ApplyDamage` (`self.GetParentActor`) Damage InstigatedBy DamageCauser (`GameplayStatics.GetObjectClass` DamageType)))

(event `self.ReceiveTick`
  (params (DeltaSeconds :type "Float (single-precision)"))
  (bind _ownercharmovementcomp (`self.OwnerCharMovementComp`))
  (`/Engine/EditorBlueprintResources/StandardMacros.IsValid` _ownercharmovementcomp
    (:`Is Valid`
      (set `self.BurstAlpha` (`KismetMathLibrary.MapRangeClamped` (`KismetMathLibrary.VSize` (`MovementComponent.Velocity` _ownercharmovementcomp)) 0.0 2000.0 0.0 1.0)))))

(fn `UserConstructionScript`)