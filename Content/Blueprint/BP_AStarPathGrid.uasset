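; Grid actor, named for A* pathfinding, that holds a node list and sizes a box volume to the grid.
; The construction script sets the Box extent from GridSize, calls the parent construction script, then runs a loop with an empty body.
; The event graph has no live logic, only an unconnected debug print of the first node's neighbour count.
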(event `self.ReceiveTick`
  (params (DeltaSeconds :type "Float (single-precision)")))

(fn `UserConstructionScript`
  (`BoxComponent.SetBoxExtent` (`self.Box`) (`self.GridSize`) true)
  (`parent.UserConstructionScript`)
  (for _ (range 16)
    _))