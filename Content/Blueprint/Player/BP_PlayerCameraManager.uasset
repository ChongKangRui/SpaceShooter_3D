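; Player camera manager that drives the view for the player ship with smoothed rotation.
; BlueprintUpdateCamera caches the camera target as BP_PlayerShip, then takes location and FOV directly from that ship's FollowCamera.
; Rotation comes from UpdateSmoothRotation, which uses RInterpTo to ease toward the ship actor's rotation each update, so the view lags slightly behind turns while position stays locked.
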(fn `BlueprintUpdateCamera`
  (params (CameraTarget :type "Actor Object Reference"))
  (returns (NewCameraLocation :type "Vector Structure") (NewCameraRotation :type "Rotator Structure") (NewCameraFOV :type "Float (single-precision)") (ReturnValue :type Boolean))
  (bind _followcamera (`SpaceShooter_Player.FollowCamera` (`self.As BP Player Ship`)))
  (`/Engine/EditorBlueprintResources/StandardMacros.IsValid` (`self.As BP Player Ship`)
    (:`Is Valid`
      (`self.Update Smooth Rotation`)
      (return (`SceneComponent.K2_GetComponentLocation` _followcamera) (`self.CurrentCamRotation`) (`CameraComponent.FieldOfView` _followcamera) true))
    (:`Is Not Valid`
      (bind _asbp_player_ship (cast `/Game/Blueprint/Player/BP_PlayerShip` CameraTarget))
      (set `self.As BP Player Ship` _asbp_player_ship))))

(fn `Update Smooth Rotation`
  (set `self.CurrentCamRotation` (`KismetMathLibrary.RInterpTo` (`self.CurrentCamRotation`) (`self.K2_GetActorRotation` (`self.As BP Player Ship`)) (`GameplayStatics.GetWorldDeltaSeconds`) 15.0))
  (return))

(fn `UserConstructionScript`)